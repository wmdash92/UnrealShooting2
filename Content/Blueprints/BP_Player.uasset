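; BP_Player is a player-controlled actor that moves in the Y-Z plane and fires bullets.
; Each tick it combines horizontal and vertical axis input into a normalized direction, scales it by MoveSpeed and delta time, and applies it as a swept location change.
; Pressing Fire1 calls FireBullet, which spawns BP_Bullet at the SpawnArrow's location and plays a blaster sound.
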(event `self.ReceiveTick`
  (params (DeltaSeconds :type "Float (single-precision)"))
  ;[1 1 1] Set Actor Location
  (`self.K2_SetActorLocation` (+ (`self.K2_GetActorLocation`) (* (* (`KismetMathLibrary.Normal` (`KismetMathLibrary.MakeVector` 0.0 (`self.GetInputAxisValue`) (`self.GetInputAxisValue`))) (`self.MoveSpeed`)) DeltaSeconds)) true))

(event `InputAction|Fire1`
  (params (Key :type "Key Structure"))
  (:`Pressed`
    (`self.FireBullet`)))

(fn `FireBullet`
  (`|SpawnActorFromClass` "/Game/Blueprints/BP_Bullet.BP_Bullet_C" (`KismetMathLibrary.MakeTransform` (`SceneComponent.K2_GetComponentLocation` (`self.SpawnArrow`))) "AlwaysSpawn" "OverrideRootScale" null null)
  (`GameplayStatics.PlaySound2D` "/Game/Sounds/star-wars-blaster.star-wars-blaster" 1.0 1.0 0.0 null null))

(fn `UserConstructionScript`)