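; BP_FlowControlTest is a test Blueprint for flow control that prints whether numbers are even or odd.
; On BeginPlay, a loop from 1 to 10 uses modulo and a branch to print a Korean even or odd message, color-coded blue or red.
; A disconnected nested-branch chain that prints random numbers never runs, and the overlap and Tick events are empty.
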(event `self.ReceiveBeginPlay`
  (for _index (range 1 11)
    (if (== (mod _index 2) 0)
      (`KismetSystemLibrary.PrintString` (`KismetStringLibrary.Concat_StrStr` "짝수" (`KismetStringLibrary.Conv_IntToString` _index) "입니다") true true (struct :`R` 0.326854 :`G` 0.755408 :`B` 1.0 :`A` 1.0) 10.0)
      (else
        (`KismetSystemLibrary.PrintString` (`KismetStringLibrary.Concat_StrStr` "홀수 " (`KismetStringLibrary.Conv_IntToString` _index) " 입니다") true true (struct :`R` 1.0 :`G` 0.136735 :`B` 0.256523 :`A` 1.0) 10.0)))))

(fn `UserConstructionScript`)