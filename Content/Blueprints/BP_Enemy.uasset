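; Enemy actor for a simple shooter that flies at the player and ends the game on contact.
; On BeginPlay it randomly picks, weighted by DirRate, straight down or the player's current position as a fixed heading, then moves along it each Tick with sweep.
; Overlapping a bullet destroys both with an explosion.
; Overlapping the player destroys both with sparks and calls EndGame, which pauses and shows the main widget and cursor.
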(event `self.ReceiveBeginPlay`
  (bind _asbp_player (cast `/Game/Blueprints/BP_Player` (`GameplayStatics.GetPlayerPawn` 0)))
  (if (< (`KismetMathLibrary.RandomIntegerInRange` 0 99) (`self.DirRate`))
    (set `self.MoveDirection` (0.0 0.0 -1.0))
    (else
      (set `self.MoveDirection` (`KismetMathLibrary.Normal` (- (`self.K2_GetActorLocation` _asbp_player) (`self.K2_GetActorLocation`)))))))

(event `self.ReceiveTick`
  (params (DeltaSeconds :type "Float (single-precision)"))
  (`self.K2_SetActorLocation` (+ (`self.K2_GetActorLocation`) (* (* (`self.MoveDirection`) (`self.MoveSpeed`)) DeltaSeconds)) true))

(event `self.ReceiveActorBeginOverlap`
  (params (OtherActor :type "Actor Object Reference"))
  (bind _asbp_player (cast `/Game/Blueprints/BP_Player` OtherActor)
    (:`then`
      (`self.K2_DestroyActor` _asbp_player)
      (`GameplayStatics.SpawnEmitterAtLocation` "/Game/StarterContent/Particles/P_Sparks.P_Sparks" (`self.K2_GetActorLocation`))
      (`self.EndGame`)
      (`self.K2_DestroyActor`)
      (`KismetSystemLibrary.PrintString` (`KismetSystemLibrary.GetObjectName` _asbp_player) true true (struct :`G` 0.66 :`B` 1.0 :`A` 1.0) 1.0))
    (:`CastFailed`
      (bind _asbp_bullet (cast `/Game/Blueprints/BP_Bullet` OtherActor))
      (`self.K2_DestroyActor` _asbp_bullet)
      (`GameplayStatics.SpawnEmitterAtLocation` "/Game/StarterContent/Particles/P_Explosion.P_Explosion" (`self.K2_GetActorLocation`) (struct))
      (`self.K2_DestroyActor`)
      (`KismetSystemLibrary.PrintString` (`KismetSystemLibrary.GetObjectName` _asbp_bullet)))))

(event `self.Box.OnComponentBeginOverlap`
  (params (OverlappedComponent :type "PrimitiveComponent Object Reference") (OtherActor :type "Actor Object Reference") (OtherComp :type "PrimitiveComponent Object Reference") (OtherBodyIndex :type Integer) (bFromSweep :type Boolean) (SweepResult :type "HitResult Structure (by ref)")))

(fn `EndGame`
  (`GameplayStatics.SetGamePaused` true)
  (set `PlayerController.bShowMouseCursor` true (`GameplayStatics.GetPlayerController` 0))
  (bind _returnvalue (`|CreateWidget` "/Game/UI/BP_MainWidget.BP_MainWidget_C"))
  (`UserWidget.AddToViewport` _returnvalue 0))

(fn `UserConstructionScript`)